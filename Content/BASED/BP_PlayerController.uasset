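; BP_PlayerController is a player controller that sets up input and opens the pause menu.
; On BeginPlay it adds the IMC_Meowfficer Enhanced Input mapping context.
; When IA_Pause starts, it pauses the game and pushes CAW_Pause onto the main widget stack.
; It then switches to UI-only input, shows the cursor and centers it in the viewport; unpausing is not handled here.
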(event `self.ReceiveBeginPlay`
  ; Mapping Context (Input)
  (`EnhancedInputSubsystemInterface.AddMappingContext` (subsystem `EnhancedInputLocalPlayerSubsystem`) "/Game/BASED/Inputs/IMC_Meowfficer.IMC_Meowfficer" 0 (struct)))

(event `EnhancedInput|/Game/BASED/Inputs/IA_Pause`
  (params (ActionValue :type Boolean) (ElapsedSeconds :type "Float (double-precision)") (TriggeredSeconds :type "Float (double-precision)") (InputAction :type "InputAction Object Reference" :default "/Game/BASED/Inputs/IA_Pause.IA_Pause"))
  (bind (_x _y) (`KismetMathLibrary.BreakVector2D` (`WidgetLayoutLibrary.GetViewportSize`)))
  (:`Started`
    (`GameplayStatics.SetGamePaused` true)
    (`CommonActivatableWidgetContainerBase.BP_AddWidget` (`/Game/BASED/Data/ML_Utils.ReturnMainStack` self) "/Game/UI/Widgets/CAW_Pause.CAW_Pause_C")
    (`WidgetBlueprintLibrary.SetInputMode_UIOnlyEx` self null "DoNotLock" true)
    (set `self.bShowMouseCursor` true)
    (`self.SetMouseLocation` (`KismetMathLibrary.FTrunc` (/ _x 2.0)) (`KismetMathLibrary.FTrunc` (/ _y 2.0)))))

(fn `UserConstructionScript`)