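; Interactable dialogue trigger component that opens dialogue when a player interacts with it.
; Interact increments the sender's CanMove counter, used as a stacking movement lock, then finds the BP_DialogManager in the level.
; It calls ShowDialog with the manager's own dialogue table and current ID, so the trigger supplies only the player.
; ReturnInteractStatus reports the IsInteractable flag, which Interact itself does not check.
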(event `/Game/BASED/Interface/BPI_Interact.interact`
  (params (Sender :type "/Game/BASED/Player/P_Meowfficer Object Reference"))
  ; Increase stop movement count
  (bind _result (`/Engine/EditorBlueprintResources/StandardMacros.IncrementInt` (`/Game/BASED/Player/P_Meowfficer.CanMove` Sender))
    (:`  `
      (set `/Game/BASED/Player/P_Meowfficer.CanMove` _result Sender)
      (bind _returnvalue (`GameplayStatics.GetActorOfClass` "/Game/Blueprints/Manager/BP_DialogManager.BP_DialogManager_C"))
      (bind _output_get (set `self.DialogManager` _returnvalue))
      (`/Game/Blueprints/Manager/BP_DialogManager.ShowDialog` _output_get (`/Game/Blueprints/Manager/BP_DialogManager.DialogTable` _output_get) (`/Game/Blueprints/Manager/BP_DialogManager.CurrentID` _output_get) Sender))))

(fn `ReturnInteractStatus`
  (returns (isInteractable :type Boolean))
  (return (`self.isInteractable`)))