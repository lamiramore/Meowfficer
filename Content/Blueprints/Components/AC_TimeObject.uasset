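; AC_TimeObject is an actor component that changes its owner's appearance and placement according to the current time period.
; It binds to the player P_Meowfficer's time-change dispatcher and applies BP_TimeManager's DebugTime on BeginPlay.
; For times keyed in the ObjectTimeState map, it teleports the owner and sets the static mesh and material.
; For other times, it hides the mesh and disables collision.
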(event `self.ReceiveBeginPlay`
  (bind _returnvalue (`GameplayStatics.GetActorOfClass` "/Game/BASED/Player/P_Meowfficer.P_Meowfficer_C"))
  (add `/Game/BASED/Player/P_Meowfficer.OnTimeChangeDispatcher` _returnvalue (delegate `OnTimeSwitched`)) ; Event From Player
  (bind _returnvalue_2 (`GameplayStatics.GetActorOfClass` "/Game/Blueprints/Manager/BP_TimeManager.BP_TimeManager_C"))
  (`self.OnTimeSwitched` (`/Game/Blueprints/Manager/BP_TimeManager.DebugTime` _returnvalue_2)))

(event `OnTimeSwitched`
  (params (CurrentTime :type "/Game/BASED/Data/E_TimeState Enum" :default "NewEnumerator0"))
  (bind _returnvalue (`self.GetOwner`))
  (bind _objecttimestate (`self.ObjectTimeState`))
  (bind _returnvalue_2 (`Actor.GetComponentByClass` (`self.GetOwner`) "/Script/Engine.StaticMeshComponent"))
  (bind _returnvalue_3 (`Actor.GetComponentByClass` (`self.GetOwner`) "/Script/Engine.StaticMeshComponent"))
  (bind _returnvalue_4 (`Actor.GetComponentByClass` _returnvalue "/Script/Engine.StaticMeshComponent"))
  (bind _keys (`BlueprintMapLibrary.Map_Keys` _objecttimestate))
  (bind _returnvalue_5 (`KismetArrayLibrary.Array_Find` _keys CurrentTime))
  (if (!= _returnvalue_5 -1)
    (`PrimitiveComponent.SetCollisionEnabled` _returnvalue_3 "QueryAndPhysics")
    (`SceneComponent.SetVisibility` _returnvalue_3 true false)
    (bind _values (`BlueprintMapLibrary.Map_Values` _objecttimestate))
    (bind (_output_transform _output_mesh _output_material) (break `/Game/BASED/Data/S_TimeObjectState` (`|GetArrayItem` _values _returnvalue_5)))
    (`Actor.K2_SetActorTransform` _returnvalue _output_transform false true)
    (`StaticMeshComponent.SetStaticMesh` _returnvalue_4 _output_mesh)
    (`PrimitiveComponent.SetMaterial` _returnvalue_4 0 _output_material)
    (else
      ; If not in current Time
      (`PrimitiveComponent.SetCollisionEnabled` _returnvalue_2 "NoCollision")
      (`SceneComponent.SetVisibility` _returnvalue_2 false false))))