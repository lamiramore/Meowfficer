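; Actor component that makes its owner inspectable as evidence in a separate 3D viewer.
; StartInspect increments the player's CanMove counter, spawns P_InspectPawn at a fixed location and feeds it evidence data, rotation, scale and a mesh, defaulting to the owner's static mesh.
; It registers the viewer on BP_PlayerController, pushes CAW_Inspect onto the main widget stack and enables cursor input.
; The widget's close event destroys the viewer, clears references and decrements CanMove.
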(event `StartInspect`
  (params (Player :type "/Game/BASED/Player/P_Meowfficer Object Reference"))
  (bind _returnvalue (`GameplayStatics.GetPlayerController` 0))
  (bind _result (`/Engine/EditorBlueprintResources/StandardMacros.IncrementInt` (`/Game/BASED/Player/P_Meowfficer.CanMove` Player))
    (:`  `
      (set `/Game/BASED/Player/P_Meowfficer.CanMove` _result Player)
      ; Update Data
      (bind (_mesh _rotationspeed _evidencedata _meshsize) (`self.GetInspectData`))
      ;; Den Inspect Actor Spawnen
      (bind _returnvalue_2 (`|SpawnActorFromClass` "/Game/Blueprints/Manager/P_InspectPawn.P_InspectPawn_C" (`KismetMathLibrary.MakeTransform` (2592.0 2844.0 -604.0)) "Undefined" "MultiplyWithRoot" null null))
      (bind _asbp_player_controller (cast `/Game/BASED/Player/BP_PlayerController` (`GameplayStatics.GetPlayerController` 0)))
      (bind _output_get (set `/Game/BASED/Player/BP_PlayerController.CurrentInspectViewer` _returnvalue_2 _asbp_player_controller)) ; set variable in player controller
      (`KismetSystemLibrary.PrintString` "Viewer Set")
      (bind _output_get_2 (set `self.CurrentInspectViewer` _returnvalue_2))
      (`/Game/Blueprints/Manager/P_InspectPawn.InspectSetup` _output_get_2 _mesh _rotationspeed _evidencedata _meshsize)
      ; Push Widget
      (bind _returnvalue_3 (`CommonActivatableWidgetContainerBase.BP_AddWidget` (`/Game/BASED/Data/ML_Utils.ReturnMainStack` _returnvalue) "/Game/UI/Widgets/CAW_Inspect.CAW_Inspect_C"))
      (bind _output_get_3 (set `self.InspectWidget` _returnvalue_3))
      (add `/Game/UI/Widgets/CAW_Inspect.OnCloseInspect` _output_get_3 (delegate `OnCloseHandler`))
      (set `PlayerController.bShowMouseCursor` true _returnvalue)
      (`WidgetBlueprintLibrary.SetInputMode_GameAndUIEx` _returnvalue _output_get_3)
      (`/Game/UI/Widgets/CAW_Inspect.UpdateEvidenceData` _returnvalue_3 _evidencedata))))

(event `OnCloseHandler`
  ; InspectPawn Destroyen
  (bind _currentinspectviewer (`self.CurrentInspectViewer`)
    (:`then`
      (`Actor.K2_DestroyActor` _currentinspectviewer)
      (set `self.InspectWidget` null)
      (bind _asbp_player_controller (cast `/Game/BASED/Player/BP_PlayerController` (`GameplayStatics.GetPlayerController` 0)))
      (set `/Game/BASED/Player/BP_PlayerController.CurrentInspectViewer` null _asbp_player_controller)
      (set `self.CurrentInspectViewer` null)
      (bind _result (`/Engine/EditorBlueprintResources/StandardMacros.DecrementInt` (`/Game/BASED/Player/P_Meowfficer.CanMove` (stale `StartInspect` Player)))
        (:`  `
          (set `/Game/BASED/Player/P_Meowfficer.CanMove` _result (stale `StartInspect` Player))
          (`KismetSystemLibrary.PrintString` "CLOSEDD"))))
    (:`else`)))

(fn `GetInspectData`
  (returns (Mesh :type "StaticMesh Object Reference") (RotationSpeed :type "Float (double-precision)") (EvidenceData :type "/Game/BASED/Data/S_EvidenceData Structure") (MeshSize :type "Vector Structure"))
  (bind _evidencedata (`self.EvidenceData`))
  (bind _meshsize (`self.MeshSize`))
  (bind _rotationspeed (`self.RotationSpeed`))
  (bind _inpectablemesh (`self.InpectableMesh`)
    (:`then`
      (bind _output_get (set `self.Mesh` _inpectablemesh))
      (return _output_get _rotationspeed _evidencedata _meshsize))
    (:`else`
      (bind _output_get_2 (set `self.Mesh` (`StaticMeshComponent.StaticMesh` (`Actor.GetComponentByClass` (`self.GetOwner`) "/Script/Engine.StaticMeshComponent"))))
      (return _output_get_2 _rotationspeed _evidencedata _meshsize))))