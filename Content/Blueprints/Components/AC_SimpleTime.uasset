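; AC_SimpleTime is an actor component that shows its owner only during certain times in a time-switching mechanic.
; On BeginPlay it binds to the P_Meowfficer player's time-change dispatcher and applies the BP_TimeManager's DebugTime as the initial state.
; Each switch checks the new time against ObjectTime, enabling the owner's visibility and collision on a match and disabling both otherwise.
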(event `self.ReceiveBeginPlay`
  (bind _returnvalue (`GameplayStatics.GetActorOfClass` "/Game/BASED/Player/P_Meowfficer.P_Meowfficer_C"))
  (add `/Game/BASED/Player/P_Meowfficer.OnTimeChangeDispatcher` _returnvalue (delegate `OnTimeSwitched`)) ; Event From Player
  (bind _returnvalue_2 (`GameplayStatics.GetActorOfClass` "/Game/Blueprints/Manager/BP_TimeManager.BP_TimeManager_C"))
  (`self.OnTimeSwitched` (`/Game/Blueprints/Manager/BP_TimeManager.DebugTime` _returnvalue_2)))

(event `OnTimeSwitched`
  (params (CurrentTime :type "/Game/BASED/Data/E_TimeState Enum" :default "NewEnumerator0"))
  (bind _returnvalue (`self.GetOwner`))
  (bind _returnvalue_2 (`self.GetOwner`))
  (if (`KismetArrayLibrary.Array_Contains` (`self.ObjectTime`) CurrentTime)
    (`Actor.SetActorHiddenInGame` _returnvalue_2 false)
    (`Actor.SetActorEnableCollision` _returnvalue_2 true)
    (else
      ; If not in current Time
      (`Actor.SetActorHiddenInGame` _returnvalue true)
      (`Actor.SetActorEnableCollision` _returnvalue false))))