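; Inspectable object pawn that the player interacts with to pull it in front of the camera and rotate it.
; Interact matches InspectCamera to the player camera, possesses this pawn, pushes the inspect widget and eases the object into view.
; While inspecting, Look drives pitch and yaw and Move drives roll on a separate rotator component.
; IA_Interact repossesses the player, restores control rotation, removes the widget and eases the object home.
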(event `self.ReceiveBeginPlay`
  (set `self.HomeRelativeTransform` (`SceneComponent.GetRelativeTransform` (`self.InspectableObjectScene`))))

(event `/Game/Blueprints/Interfaces/BPI_Interact.Interact`
  (params (PlayerRef :type "/Game/Blueprints/Framework/BP_Player Object Reference"))
  (bind (_returnvalue_location _returnvalue_rotation) (`KismetMathLibrary.BreakTransform` (`SceneComponent.GetRelativeTransform` (`self.InspectCamera`))))
  (set `self.Player Ref` PlayerRef)
  (if (not (`self.AllowInspectInput`))
    (set `self.ControlRotation` (`Controller.GetControlRotation` (`GameplayStatics.GetPlayerController` 0)))
    (`SceneComponent.K2_SetWorldTransform` (`self.InspectCamera`) (`SceneComponent.K2_GetComponentToWorld` (`/Game/Blueprints/Framework/BP_Player.Camera` (`self.Player Ref`))) false true)
    (`Controller.Possess` (`GameplayStatics.GetPlayerController` 0) self)
    (bind _returnvalue (`CommonActivatableWidgetContainerBase.BP_AddWidget` (`/Game/Blueprints/Librarys/FL_Miscellaneous.ReturnMainStack` (`GameplayStatics.GetPlayerController` 0)) "/Game/Blueprints/UI/CAW_Inspect.CAW_Inspect_C"))
    (set `self.InspectWidgetInstance` _returnvalue)
    (`KismetSystemLibrary.MoveComponentTo` (`self.InspectableObjectScene`) (+ _returnvalue_location (* (`KismetMathLibrary.GetForwardVector` _returnvalue_rotation) (`self.InspectDistance`))) _returnvalue_rotation true true (`self.InspectInDuration`) true)
    (set `self.AllowInspectInput` true)))

(event `EnhancedInput|/Game/Input/IA_Interact`
  (params (ActionValue :type Boolean) (ElapsedSeconds :type "Float (double-precision)") (TriggeredSeconds :type "Float (double-precision)") (InputAction :type "InputAction Object Reference" :default "/Game/Input/IA_Interact.IA_Interact"))
  (bind (_homerelativetransform_location _homerelativetransform_rotation) (`KismetMathLibrary.BreakTransform` (`self.HomeRelativeTransform`)))
  (:`Triggered`
    (if (`self.AllowInspectInput`)
      (set `self.AllowInspectInput` false)
      (`Controller.Possess` (`GameplayStatics.GetPlayerController` 0) (`self.Player Ref`))
      (`Controller.SetControlRotation` (`GameplayStatics.GetPlayerController` 0) (`self.ControlRotation`))
      (`CommonActivatableWidgetContainerBase.RemoveWidget` (`/Game/Blueprints/Librarys/FL_Miscellaneous.ReturnMainStack` (`GameplayStatics.GetPlayerController` 0)) (`self.InspectWidgetInstance`))
      (`|ExecutionSequence`
        (:`then_0`
          (`KismetSystemLibrary.MoveComponentTo` (`self.InspectableObjectScene`) _homerelativetransform_location _homerelativetransform_rotation true true (* (`self.InspectInDuration`) 1.5) true))
        (:`then_1`
          (`KismetSystemLibrary.MoveComponentTo` (`self.InspectableObjectRotator`) (0.0 0.0 0.0) (struct) true true (* (`self.InspectInDuration`) 1.5) true))))))

(event `EnhancedInput|/Game/Input/IA_Look`
  (params (ActionValue :type "Vector2D Structure") (ElapsedSeconds :type "Float (double-precision)") (TriggeredSeconds :type "Float (double-precision)") (InputAction :type "InputAction Object Reference" :default "/Game/Input/IA_Look.IA_Look"))
  (:`Triggered`
    (if (`self.AllowInspectInput`)
      (`SceneComponent.K2_SetRelativeRotation` (`self.InspectableObjectRotator`) (`KismetMathLibrary.ComposeRotators` (`SceneComponent.RelativeRotation` (`self.InspectableObjectRotator`)) (`KismetMathLibrary.MakeRotator` 0.0 (* ActionValue_Y 3.0) (* ActionValue_X -3.0))) false false))))

(event `EnhancedInput|/Game/Input/IA_Move`
  (params (ActionValue :type "Vector2D Structure") (ElapsedSeconds :type "Float (double-precision)") (TriggeredSeconds :type "Float (double-precision)") (InputAction :type "InputAction Object Reference" :default "/Game/Input/IA_Move.IA_Move"))
  (:`Triggered`
    (if (`self.AllowInspectInput`)
      (`SceneComponent.K2_SetRelativeRotation` (`self.InspectableObjectRotator`) (`KismetMathLibrary.ComposeRotators` (`SceneComponent.RelativeRotation` (`self.InspectableObjectRotator`)) (`KismetMathLibrary.MakeRotator` (* ActionValue_X 3.0))) false false))))

(fn `ReturnInteractStatus`
  (returns (IsInteractable :type Boolean) (Type :type "/Game/Blueprints/Interfaces/E_InteractableTypes Enum"))
  (return true "NewEnumerator2"))

(fn `UserConstructionScript`)