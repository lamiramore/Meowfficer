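; Base actor, by its name, for objects that change or disappear when the game's time switches.
; On BeginPlay it binds to the time change dispatcher on P_Meowfficer.
; Each switch looks up the time in ObjectTimeState, applying that entry's transform, mesh and material, or hiding the mesh and disabling collision if none exists.
; Initial visibility logic based on BP_TimeManager's DebugTime is disconnected in both graphs.
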(event `self.ReceiveBeginPlay`
  (bind _returnvalue (`GameplayStatics.GetActorOfClass` "/Game/BASED/Player/P_Meowfficer.P_Meowfficer_C"))
  (add `/Game/BASED/Player/P_Meowfficer.OnTimeChangeDispatcher` _returnvalue (delegate `OnTimeSwitched`)))

(event `OnTimeSwitched`
  (params (CurrentTime :type "/Game/BASED/Data/E_TimeState Enum" :default "NewEnumerator0"))
  (bind _mesh (`self.Mesh`))
  (bind _objecttimestate (`self.ObjectTimeState`))
  (bind _keys (`BlueprintMapLibrary.Map_Keys` _objecttimestate))
  (bind _returnvalue (`KismetArrayLibrary.Array_Find` _keys CurrentTime))
  (if (!= _returnvalue -1)
    (`PrimitiveComponent.SetCollisionEnabled` (`self.Mesh`) "QueryAndPhysics")
    (`SceneComponent.SetVisibility` (`self.Mesh`) true false)
    (bind _values (`BlueprintMapLibrary.Map_Values` _objecttimestate))
    (bind (_output_transform _output_mesh _output_material) (break `/Game/BASED/Data/S_TimeObjectState` (`|GetArrayItem` _values _returnvalue)))
    (`self.K2_SetActorTransform` _output_transform false true)
    (`StaticMeshComponent.SetStaticMesh` _mesh _output_mesh)
    (`PrimitiveComponent.SetMaterial` _mesh 0 _output_material)
    (else
      (`PrimitiveComponent.SetCollisionEnabled` (`self.Mesh`) "NoCollision")
      (`SceneComponent.SetVisibility` (`self.Mesh`) false false))))

(fn `UserConstructionScript`
  (bind _returnvalue (`GameplayStatics.GetActorOfClass` "/Game/Blueprints/BP_TimeManager.BP_TimeManager_C")) ; Holt sich die anfangszeit des levels
)