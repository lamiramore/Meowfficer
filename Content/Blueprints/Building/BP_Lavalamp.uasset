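; BP_Lavalamp is a lava lamp whose point light continuously blends through an array of colors.
; On BeginPlay, the ColorSwitch timeline lerps the light from the current color to the next.
; When the timeline finishes, it advances the wrapping color index, shifts the color pair and restarts itself, looping endlessly.
; An intensity-modulation node is left unconnected, so the graph only animates color.
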(event `self.ReceiveBeginPlay`
  (set `self.CurrentColor` (`|GetArrayItem` (`self.Colors`)))
  (set `self.NextColor` (`|GetArrayItem` (`self.Colors`) 1))
  (bind (_direction _alpha _intensity) (`Timeline|ColorSwitch` :!label _label)
    (:`Update`
      (`LightComponent.SetLightColor` (`self.PointLight`) (`KismetMathLibrary.LinearColorLerp` (`self.CurrentColor`) (`self.NextColor`) _alpha) true))
    (:`Finished`
      (bind _result (`/Engine/EditorBlueprintResources/StandardMacros.IncrementInt` (`self.CurrentColorIndex`))
        (:`  `
          (bind _output_get (set `self.CurrentColorIndex` (mod _result (`KismetArrayLibrary.Array_Length` (`self.Colors`)))))
          (set `self.CurrentColor` (`self.NextColor`))
          (set `self.NextColor` (`|GetArrayItem` (`self.Colors`) _output_get))
          (goto _label :!via `PlayFromStart`))))))

(fn `UserConstructionScript`)