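; BP_TP is an interactable teleport point, built around a BalconyDoor mesh, that moves the interacting actor to a set transform.
; Interact pushes a configurable widget onto the player's main UI stack, waits briefly, teleports the sender, then removes the widget and restores game-only input with the cursor hidden.
; Interaction events track an Interactable flag, which React switches on, and toggle an outline overlay material on the door for highlighting.
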(event `/Game/BASED/Interface/BPI_Interact.SetInteractStatus`
  (params (isInteractable :type Boolean))
  (set `self.interactable` isInteractable))

(event `/Game/BASED/Interface/BPI_React.React`
  (params (Solved :type Boolean))
  (`self.SetInteractStatus` true))

(event `/Game/BASED/Interface/BPI_Interact.interact`
  (params (Sender :type "/Game/BASED/Player/P_Meowfficer Object Reference"))
  (bind _returnvalue (`GameplayStatics.GetPlayerController` 0))
  (`/Engine/EditorBlueprintResources/StandardMacros.IsValid` Sender
    (:`Is Valid`
      (bind _returnvalue_2 (`CommonActivatableWidgetContainerBase.BP_AddWidget` (`/Game/BASED/Data/ML_Utils.ReturnMainStack` (`GameplayStatics.GetPlayerController` 0)) (`self.WidgetToOpen`)))
      (`KismetSystemLibrary.Delay` 1.5)
      (`self.K2_SetActorTransform` Sender (`self.NewTransform`) false true)
      (set `PlayerController.bShowMouseCursor` false (`GameplayStatics.GetPlayerController` 0))
      (`CommonActivatableWidgetContainerBase.RemoveWidget` (`/Game/BASED/Data/ML_Utils.ReturnMainStack` _returnvalue) _returnvalue_2)
      (`WidgetBlueprintLibrary.SetInputMode_GameOnly` _returnvalue true))))

(event `/Game/BASED/Interface/BPI_Interact.UpdateHighlight`
  (params (highlightActive :type Boolean))
  (bind _balconydoor (`self.BalconyDoor`))
  ; Highlight
  (if highlightActive
    (`MeshComponent.SetOverlayMaterial` _balconydoor "/Game/GameArt/Materials/Outline/MI_InteractOutline.MI_InteractOutline")
    (else
      (`MeshComponent.SetOverlayMaterial` _balconydoor null))))

(fn `ReturnInteractStatus`
  (returns (isInteractable :type Boolean))
  (return (`self.interactable`)))

(fn `UserConstructionScript`)