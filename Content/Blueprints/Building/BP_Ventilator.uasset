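; BP_Ventilator is a building fan that spins a CubeRotator component around yaw, starting on BeginPlay if Defaultrotation is set or through StartRotate.
; The RotateVentilator timeline scales RotationSpeed by its Speed track for local rotation, then hands off to a looping timer that calls Rotating for constant world-space spin.
; IsRotating guards against restarts, printing a debug string on repeat calls; nothing here stops the rotation.
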(event `self.ReceiveBeginPlay`
  (if (`self.defaultrotation`)
    (`self.StartRotate`)))

(event `StartRotate`
  (if (`self.isRotating`)
    (`KismetSystemLibrary.PrintString` "uuuiiiiaaiiuuiiaaii")
    (else
      (set `self.isRotating` true)
      (bind (_direction _speed) (`Timeline|RotateVentilator`)
        (:`Update`
          (`SceneComponent.K2_AddLocalRotation` (`self.CubeRotator`) (`KismetMathLibrary.MakeRotator` 0.0 0.0 (* (* _speed (`self.RotationSpeed`)) (`GameplayStatics.GetWorldDeltaSeconds`))) false false))
        (:`Finished`
          (`KismetSystemLibrary.K2_SetTimer` null "Rotating" 0.016 true true))))))

(fn `Rotating`
  (`SceneComponent.K2_AddWorldRotation` (`self.CubeRotator`) (`KismetMathLibrary.MakeRotator` 0.0 0.0 (* (`self.RotationSpeed`) (`GameplayStatics.GetWorldDeltaSeconds`))) false false))

(fn `UserConstructionScript`)