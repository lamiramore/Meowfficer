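; Dialog manager that opens the dialog UI for a player and feeds it lines from a data table.
; ShowDialog pushes CAW_Dialogsystem onto the main widget stack, enables Game and UI input with a cursor, and passes the player and manager references.
; LoadDialogLine looks up a DialogTable row by ID, stores it as CurrentLine and sends it to the widget's UpdateDialog.
; TypeWriter is an empty stub, and debug prints remain.
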(event `ShowDialog`
  (params (StartID :type Name) (Player :type "/Game/BASED/Player/P_Meowfficer Object Reference"))
  (bind _returnvalue (`GameplayStatics.GetPlayerController` 0))
  ; Erster Dialogblock Start
  (bind _returnvalue_2 (`CommonActivatableWidgetContainerBase.BP_AddWidget` (`/Game/BASED/Data/ML_Utils.ReturnMainStack` (`GameplayStatics.GetPlayerController` 0)) "/Game/UI/Widgets/CAW_Dialogsystem.CAW_Dialogsystem_C"))
  (bind _output_get (set `self.DialogWidget` _returnvalue_2))
  (`WidgetBlueprintLibrary.SetInputMode_GameAndUIEx` _returnvalue null "DoNotLock" true true)
  (set `PlayerController.bShowMouseCursor` true _returnvalue)
  (`/Engine/EditorBlueprintResources/StandardMacros.IsValid` (`/Game/UI/Widgets/CAW_Dialogsystem.DialogManagerRef` _output_get)
    (:`Is Valid`
      _)
    (:`Is Not Valid`
      (set `/Game/UI/Widgets/CAW_Dialogsystem.DialogManagerRef` self _returnvalue_2)))
  (set `/Game/UI/Widgets/CAW_Dialogsystem.Player` Player _output_get)
  (`self.LoadDialogLine` StartID)
  (`KismetSystemLibrary.PrintString` "YAP NICHT SO VIEL FEY"))

(event `TypeWriter`)

(fn `LoadDialogLine`
  (params (RowID :type Name))
  (`KismetSystemLibrary.PrintString` "Ziehe Koksline")
  (bind _returnvalue (`|GetDataTableRow` (`self.DialogTable`) RowID)
    (:`then`
      (bind _output_get (set `self.CurrentLine` _returnvalue))
      (`/Game/UI/Widgets/CAW_Dialogsystem.UpdateDialog` (`self.DialogWidget`) _output_get)
      (`KismetSystemLibrary.PrintString` "LADE DIALOG"))
    (:`RowNotFound`
      (`KismetSystemLibrary.PrintString` "Koks nicht gefunden"))))

(fn `UserConstructionScript`)