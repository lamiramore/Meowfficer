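; BP_ChessManager manages a chessboard puzzle's sockets and can restore its starting layout.
; On BeginPlay it records each socket with the BP_ChessFigure it holds as a start state, printing an error when a socket's collectible is not a chess figure.
; Its React event resets the board by telling every recorded socket to return to its starting figure.
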(event `self.ReceiveBeginPlay`
  (for _array_element (`self.Sockets`)
    (bind _asbp_chess_figure (cast `/Game/Blueprints/Collectable/BP_ChessFigure` (`/Game/Blueprints/Collectable/BP_CollectableSocketChess.CurrentCollectible` _array_element))
      (:`then`
        (`KismetArrayLibrary.Array_Add` (`self.StartStates`) (make `/Game/BASED/Data/S_ChessStartpos` _array_element _asbp_chess_figure)))
      (:`CastFailed`
        (`KismetSystemLibrary.PrintString` "error with chessboard")))))

(event `/Game/BASED/Interface/BPI_React.React`
  (params (Solved :type Boolean))
  (`self.ResetChessboard` null))

(fn `ResetChessboard`
  (params (NewFigure :type "/Game/Blueprints/Collectable/BP_ChessFigure Object Reference"))
  (for _array_element (`self.StartStates`)
    (bind (_socket _childfigure) (break `/Game/BASED/Data/S_ChessStartpos` _array_element))
    (`/Game/Blueprints/Collectable/BP_CollectableSocketChess.ResetToStartFigure` _socket _childfigure)))

(fn `UserConstructionScript`)