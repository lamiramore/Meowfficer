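; BP_UIOpener is an interactable that opens a configurable UI widget when a P_Meowfficer interacts with it.
; Interact pauses the game and adds WidgetToOpen to the player's main widget stack.
; It then switches to UI-only input focused on that widget, shows the cursor and centers it in the viewport.
; ReturnInteractStatus exposes the IsInteractable flag.
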(event `/Game/BASED/Interface/BPI_Interact.interact`
  (params (Sender :type "/Game/BASED/Player/P_Meowfficer Object Reference"))
  (bind _returnvalue (`GameplayStatics.GetPlayerController` 0))
  (bind (_x _y) (`KismetMathLibrary.BreakVector2D` (`WidgetLayoutLibrary.GetViewportSize`)))
  (bind _asp_meowfficer (cast `/Game/BASED/Player/P_Meowfficer` Sender))
  (`/Engine/EditorBlueprintResources/StandardMacros.IsValid` _asp_meowfficer
    (:`Is Valid`
      (`GameplayStatics.SetGamePaused` true)
      (bind _returnvalue_2 (`CommonActivatableWidgetContainerBase.BP_AddWidget` (`/Game/BASED/Data/ML_Utils.ReturnMainStack` _returnvalue) (`self.WidgetToOpen`)))
      (`WidgetBlueprintLibrary.SetInputMode_UIOnlyEx` _returnvalue _returnvalue_2 "DoNotLock" true)
      (set `PlayerController.bShowMouseCursor` true _returnvalue)
      (`PlayerController.SetMouseLocation` _returnvalue (`KismetMathLibrary.FTrunc` (/ _x 2.0)) (`KismetMathLibrary.FTrunc` (/ _y 2.0))))))

(fn `ReturnInteractStatus`
  (returns (isInteractable :type Boolean))
  (return (`self.isInteractable`)))

(fn `UserConstructionScript`)