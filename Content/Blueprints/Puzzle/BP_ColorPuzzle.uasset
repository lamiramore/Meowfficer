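; BP_ColorPuzzle is an interactable puzzle piece that cycles its cylinder's material and counts as solved at a target index.
; Each interaction advances through MaterialRotation with wraparound, then sends ReactMessage to ActorsToReact with true on the solved index, or false when leaving it.
; It exposes interactable and solved status to callers and shows hover-style highlighting through an outline overlay material.
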(event `/Game/BASED/Interface/BPI_Interact.SetInteractStatus`
  (params (isInteractable :type Boolean))
  (set `self.IsInteractable` isInteractable))

(event `self.ReceiveBeginPlay`
  ; Startmaterial setzen
  (bind _output_get (set `self.CurrentMaterialIndex` (`self.StartMaterialIndex`)))
  (`PrimitiveComponent.SetMaterial` (`self.Cylinder`) 0 (`|GetArrayItem` (`self.MaterialRotation`) _output_get)))

(event `/Game/BASED/Interface/BPI_Interact.interact`
  (params (Sender :type "/Game/BASED/Player/P_Meowfficer Object Reference"))
  (bind _materialrotation (`self.MaterialRotation`))
  (bind _result (`/Engine/EditorBlueprintResources/StandardMacros.IncrementInt` (`self.CurrentMaterialIndex`))
    (:`  `
      (bind _output_get (set `self.CurrentMaterialIndex` (mod _result (`KismetArrayLibrary.Array_Length` _materialrotation))))
      (`PrimitiveComponent.SetMaterial` (`self.Cylinder`) 0 (`|GetArrayItem` _materialrotation _output_get))
      (if (== (`self.CurrentMaterialIndex`) (`self.SolvedIndex`))
        (set `self.Solved` true)
        (message `/Game/BASED/Interface/BPI_React.React` (`self.ActorsToReact`) true)
        (`KismetSystemLibrary.PrintString` "SOLVEDD")
        (else
          (`self.Solved`
            (:`then`
              (set `self.Solved` false)
              (message `/Game/BASED/Interface/BPI_React.React` (`self.ActorsToReact`) false))
            (:`else`)))))))

(event `/Game/BASED/Interface/BPI_Interact.UpdateHighlight`
  (params (highlightActive :type Boolean))
  (bind _cylinder (`self.Cylinder`))
  (if highlightActive
    (`MeshComponent.SetOverlayMaterial` _cylinder "/Game/GameArt/Materials/Outline/MI_InteractOutline.MI_InteractOutline")
    (else
      (`MeshComponent.SetOverlayMaterial` _cylinder null))))

(fn `ReturnInteractStatus`
  (returns (isInteractable :type Boolean))
  (return (`self.IsInteractable`)))

(fn `ReturnSolvedStatus`
  (returns (Solved :type Boolean))
  (return (`self.Solved`)))

(fn `UserConstructionScript`)