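; BP_RotationPuzzle is an interactable puzzle piece that rotates through preset orientations until it reaches its solved one.
; Each Interact advances a wrapping index into RotationSteps and sets RotationScene's relative rotation, which the construction script also applies.
; Matching SolvedPositionIndex sets Solved and signals ActorToReact through ReactMessage, while a guarded mismatch branch sends false.
; Getters expose the solved and interactable states.
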(event `/Game/BASED/Interface/BPI_Interact.interact`
  (params (Sender :type "/Game/BASED/Player/P_Meowfficer Object Reference"))
  (bind _returnvalue (+ (`self.currentPositionIndex`) 1))
  (set `self.currentPositionIndex` (`KismetMathLibrary.SelectInt` 0 _returnvalue (> _returnvalue (`KismetArrayLibrary.Array_LastIndex` (`self.RotationSteps`)))))
  (`SceneComponent.K2_SetRelativeRotation` (`self.Rotation scene`) (`|GetArrayItem` (`self.RotationSteps`) (`self.currentPositionIndex`)) false false)
  ; Set Solved
  (if (== (`self.solvedPositionIndex`) (`self.currentPositionIndex`))
    (set `self.Solved` true)
    (message `/Game/BASED/Interface/BPI_React.React` (`self.ActorToReact`) true)
    (`KismetSystemLibrary.PrintString` "DU BIST FERTIG BITCH")
    (else
      (`self.Solved`
        (:`then`
          (set `self.Solved` false)
          (message `/Game/BASED/Interface/BPI_React.React` (`self.ActorToReact`) false))
        (:`else`)))))

(event `/Game/BASED/Interface/BPI_Interact.SetInteractStatus`
  (params (isInteractable :type Boolean))
  (set `self.isInteractable` isInteractable))

(fn `ReturnInteractStatus`
  (returns (isInteractable :type Boolean))
  (return (`self.isInteractable`)))

(fn `ReturnSolvedStatus`
  (returns (Solved :type Boolean))
  (return (`self.Solved`)))

(fn `UserConstructionScript`
  (`SceneComponent.K2_SetRelativeRotation` (`self.Rotation scene`) (`|GetArrayItem` (`self.RotationSteps`) (`self.currentPositionIndex`)) false false))