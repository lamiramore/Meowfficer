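; Red collectible puzzle object that tags itself with a RedBall ID at construction on top of its parent's setup.
; Interacting disables further interaction, eases its ScaleScene component up and back to zero relative location, then re-enables interaction.
; It always reports unsolved, and a debug print with the parent Interact call is left disconnected.
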(event `/Game/BASED/Interface/BPI_Interact.interact`
  (params (Sender :type "Actor Object Reference"))
  (bind _scalescene (`self.ScaleScene`))
  (set `self.Is Interactable` false)
  (`KismetSystemLibrary.MoveComponentTo` _scalescene (0.0 0.0 150.0) (struct) true true 1.0)
  (`KismetSystemLibrary.MoveComponentTo` _scalescene (0.0 0.0 0.0) (struct) true true 1.0)
  (set `self.Is Interactable` true))

(fn `ReturnSolvedStatus`
  (returns (Solved :type Boolean))
  (return false))

(fn `UserConstructionScript`
  (`parent.UserConstructionScript`)
  (set `self.ID` "RedBall"))