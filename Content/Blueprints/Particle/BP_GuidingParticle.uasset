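; BP_GuidingParticle is a particle actor set up to travel along a spline, with a React event that responds to a Solved flag.
; On the first solved call, React deactivates the particle and sets the timeline's play rate from spline length and Speed.
; The timeline update lerps distance along the spline to position the particle in world space, but no event in the graph starts it.
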(event `/Game/BASED/Interface/BPI_React.React`
  (params (Solved :type Boolean))
  (if Solved
    (`/Engine/EditorBlueprintResources/StandardMacros.DoOnce` false
      (:`Completed`
        (`ActorComponent.SetActive` (`self.Particle`) false false)
        (`TimelineComponent.SetPlayRate` (`self.ParticleTimeline`) (/ 1.0 (/ (`SplineComponent.GetSplineLength` (`self.Spline`)) (`self.Speed`))))))))

(fn `UserConstructionScript`)