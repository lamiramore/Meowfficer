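; BP_Collectible is an interactable item that a P_Meowfficer can pick up and hold, one at a time.
; On Interact, if the sender holds no valid collectible, it disables mesh collision, waits a tick, then registers itself as HeldCollectible.
; It then snaps onto the pawn's CollectiblePivot and turns off shadow casting.
; ReturnInteractStatus exposes the IsInteractable flag; the file has no drop logic.
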(event `/Game/BASED/Interface/BPI_Interact.interact`
  (params (Sender :type "Actor Object Reference"))
  (bind _mesh (`self.Mesh`))
  (bind _asp_meowfficer (cast `/Game/BASED/Player/P_Meowfficer` Sender))
  (`/Game/BASED/Player/P_Meowfficer.HeldCollectible` _asp_meowfficer
    (:`then`)
    (:`else`
      (`PrimitiveComponent.SetCollisionEnabled` (`self.Mesh`) "NoCollision")
      (`KismetSystemLibrary.DelayUntilNextTick`)
      (set `/Game/BASED/Player/P_Meowfficer.HeldCollectible` self _asp_meowfficer)
      (`self.K2_AttachToComponent` (`/Game/BASED/Player/P_Meowfficer.CollectiblePivot` _asp_meowfficer) "None" "SnapToTarget" "SnapToTarget" "SnapToTarget")
      (`PrimitiveComponent.SetCastShadow` _mesh false)
      (`PrimitiveComponent.SetCollisionEnabled` _mesh "NoCollision"))))

(fn `ReturnInteractStatus`
  (returns (isInteractable :type Boolean))
  (return (`self.Is Interactable`)))

(fn `UserConstructionScript`)