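; BP_Movable is an interactable world object that moves its MoveScene component between a starting pose and a target transform.
; It caches the starting relative transform on BeginPlay, and each interaction uses a FlipFlop to pick the destination for an eased, timed MoveComponentTo.
; Interaction is disabled when the move begins and restored afterward unless the MoveOnce check blocks it, with the current state exposed through ReturnInteractStatus.
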(event `self.ReceiveBeginPlay`
  (set `self.StartTransform` (`SceneComponent.GetRelativeTransform` (`self.MoveScene`))))

(event `/Game/BASED/Interface/BPI_Interact.interact`
  (params (Sender :type "Actor Object Reference"))
  (set `self.isInteractible` false)
  (bind _isa (`/Engine/EditorBlueprintResources/StandardMacros.FlipFlop`)
    (:`A`
      _)
    (:`B`
      _))
  (`KismetSystemLibrary.MoveComponentTo` (`self.MoveScene`) (.location (`KismetMathLibrary.SelectTransform` (`self.TargetTransform`) (`self.StartTransform`) _isa)) (.rotation (`KismetMathLibrary.SelectTransform` (`self.TargetTransform`) (`self.StartTransform`) _isa)) true true (`self.MoveDuration`))
  (`self.MoveOnce`
    (:`then`)
    (:`else`
      (set `self.isInteractible` true))))

(fn `ReturnInteractStatus`
  (returns (isInteractable :type Boolean))
  (return (`self.isInteractible`)))

(fn `UserConstructionScript`)