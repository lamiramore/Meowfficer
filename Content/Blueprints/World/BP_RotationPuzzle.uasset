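; BP_RotationPuzzle is an interactable puzzle piece that rotates through preset steps and signals another actor when it reaches its solved position.
; Each Interact advances the index with wraparound and snaps RotationScene to that rotation; the construction script applies the starting step.
; The solved step sends ReactMessage true to ActorToReact and resets a DoOnce, which limits the false message to once upon leaving it.
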(event `/Game/BASED/Interface/BPI_Interact.interact`
  (params (Sender :type "Actor Object Reference"))
  (bind _returnvalue (+ (`self.currentPositionIndex`) 1))
  (set `self.currentPositionIndex` (`KismetMathLibrary.SelectInt` 0 _returnvalue (> _returnvalue (`KismetArrayLibrary.Array_LastIndex` (`self.RotationSteps`)))))
  (`SceneComponent.K2_SetRelativeRotation` (`self.Rotation scene`) (`|GetArrayItem` (`self.RotationSteps`) (`self.currentPositionIndex`)) false false)
  (if (== (`self.solvedPositionIndex`) (`self.currentPositionIndex`))
    (message `/Game/BASED/Interface/BPI_React.React` (`self.ActorToReact`) true)
    (goto _label :!via `Reset`)
    (else
      (`/Engine/EditorBlueprintResources/StandardMacros.DoOnce` true :!label _label
        (:`Completed`
          (message `/Game/BASED/Interface/BPI_React.React` (`self.ActorToReact`) false))))))

(fn `ReturnInteractStatus`
  (returns (isInteractable :type Boolean))
  (return (`self.isInteractable`)))

(fn `UserConstructionScript`
  (`SceneComponent.K2_SetRelativeRotation` (`self.Rotation scene`) (`|GetArrayItem` (`self.RotationSteps`) (`self.currentPositionIndex`)) false false))