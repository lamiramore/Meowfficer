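; BP_Evidence is an interactable evidence actor that can be inspected.
; On BeginPlay it looks up its EvidenceRowName row in DT_EvidenceBoardEntrys and copies that EvidenceData into its AC_Inspectable component.
; Interact hands the sender to the component's StartInspect, while a settable IsInteractable flag reports interaction status.
; A disconnected loop over the table's row names never runs.
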(event `/Game/BASED/Interface/BPI_Interact.SetInteractStatus`
  (params (isInteractable :type Boolean))
  (set `self.isInteractable` isInteractable))

(event `self.ReceiveBeginPlay`
  (bind _returnvalue (`|GetDataTableRow` "/Game/BASED/Inspect/DT_EvidenceBoardEntrys.DT_EvidenceBoardEntrys" (`.RowName` (break `DataTableRowHandle` (`self.EvidenceRowName`))))
    (:`then`
      (set `/Game/Blueprints/Components/AC_Inspectable.EvidenceData` (`.EvidenceData_2_67AFED464B2CCD0CCBC44190B41D3070` (break `/Game/BASED/Inspect/S_EvidenceBoardData` _returnvalue)) (`self.GetComponentByClass` "/Game/Blueprints/Components/AC_Inspectable.AC_Inspectable_C")))))

(event `/Game/BASED/Interface/BPI_Interact.interact`
  (params (Sender :type "/Game/BASED/Player/P_Meowfficer Object Reference"))
  ; Interact
  (`/Game/Blueprints/Components/AC_Inspectable.StartInspect` (`self.GetComponentByClass` "/Game/Blueprints/Components/AC_Inspectable.AC_Inspectable_C") Sender))

(fn `ReturnInteractStatus`
  (returns (isInteractable :type Boolean))
  (return (`self.isInteractable`)))

(fn `UserConstructionScript`)