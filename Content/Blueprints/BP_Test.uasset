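; Test actor whose Cone exists only in one time state, appearing or disappearing as the level time switches.
; At BeginPlay it binds to the time-change dispatcher on P_Meowfficer and sets its initial state from BP_TimeManager's DebugTime.
; When the time matches its ObjectTimeState, the Cone is visible and collidable; otherwise both are off.
; The construction script applies the same check to visibility only, leaving collision untouched.
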(event `self.ReceiveBeginPlay`
  (bind _returnvalue (`GameplayStatics.GetActorOfClass` "/Game/BASED/Player/P_Meowfficer.P_Meowfficer_C"))
  (add `/Game/BASED/Player/P_Meowfficer.OnTimeChangeDispatcher` _returnvalue (delegate `OnTimeSwitched`))
  (bind _returnvalue_2 (`GameplayStatics.GetActorOfClass` "/Game/Blueprints/BP_TimeManager.BP_TimeManager_C"))
  (if (`|EnumEquality` (`/Game/Blueprints/BP_TimeManager.DebugTime` _returnvalue_2) (`self.ObjectTimeState`))
    (`PrimitiveComponent.SetCollisionEnabled` (`self.Cone`) "QueryAndPhysics")
    (`SceneComponent.SetVisibility` (`self.Cone`) true false)
    (else
      (`PrimitiveComponent.SetCollisionEnabled` (`self.Cone`) "NoCollision")
      (`SceneComponent.SetVisibility` (`self.Cone`) false false))))

(event `OnTimeSwitched`
  (params (CurrentTime :type "/Game/BASED/Data/E_TimeState Enum" :default "NewEnumerator0"))
  (if (`|EnumEquality` CurrentTime (`self.ObjectTimeState`))
    (`PrimitiveComponent.SetCollisionEnabled` (`self.Cone`) "QueryAndPhysics")
    (`SceneComponent.SetVisibility` (`self.Cone`) true false)
    (else
      (`PrimitiveComponent.SetCollisionEnabled` (`self.Cone`) "NoCollision")
      (`SceneComponent.SetVisibility` (`self.Cone`) false false))))

(fn `UserConstructionScript`
  (bind _returnvalue (`GameplayStatics.GetActorOfClass` "/Game/Blueprints/BP_TimeManager.BP_TimeManager_C")) ; Holt sich die anfangszeit des levels
  (if (`|EnumEquality` (`/Game/Blueprints/BP_TimeManager.DebugTime` _returnvalue) (`self.ObjectTimeState`)) :!pinned true
    (`SceneComponent.SetVisibility` (`self.Cone`) true false)
    (else
      (`SceneComponent.SetVisibility` (`self.Cone`) false false))))