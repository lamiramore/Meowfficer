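; Inspectable time object that the player can interact with, built on a parent that handles time switching.
; Interact stores ObjectScene's relative transform as home, then, if inspect input is allowed, saves the control rotation, snaps InspectCamera to the sender's camera and calls Possess on the player controller.
; Time switches forward a fixed enum value to the parent, and interact status reports IsInteractable.
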(event `self.OnTimeSwitched`
  (params (CurrentTime :type "/Game/BASED/Data/E_TimeState Enum" :default "NewEnumerator0"))
  (`parent.OnTimeSwitched` "NewEnumerator0"))

(event `/Game/BASED/Interface/BPI_Interact.interact`
  (params (Sender :type "/Game/BASED/Player/P_Meowfficer Object Reference"))
  (set `self.Sender` Sender)
  (set `self.HomeRelativeTransform` (`SceneComponent.GetRelativeTransform` (`self.ObjectScene`))) ; Set Default Transform
  (if (`self.AllowInspectInput`)
    (set `self.ControlRotation` (`Controller.GetControlRotation` (`GameplayStatics.GetPlayerController` 0)))
    (`SceneComponent.K2_SetWorldTransform` (`self.InspectCamera`) (`SceneComponent.K2_GetComponentToWorld` (`/Game/BASED/Player/P_Meowfficer.Camera` (`self.Sender`))) false true)
    (`Controller.Possess` (`GameplayStatics.GetPlayerController` 0) null)))

(fn `ReturnInteractStatus`
  (returns (isInteractable :type Boolean))
  (return (`self.isInteractable`)))

(fn `UserConstructionScript`
  (`parent.UserConstructionScript`))