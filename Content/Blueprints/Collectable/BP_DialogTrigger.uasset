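; BP_DialogTrigger is an interactable object that starts a dialog when a player interacts with it.
; Interact increments the sender's CanMove stop-movement counter, then finds BP_DialogManager in the level and calls ShowDialog with StartRowID and the sender.
; It toggles an outline overlay material on its mesh for highlighting and exposes getters for its solved and interactable states.
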(event `/Game/BASED/Interface/BPI_Interact.interact`
  (params (Sender :type "/Game/BASED/Player/P_Meowfficer Object Reference"))
  ; Increase stop movement count
  (bind _result (`/Engine/EditorBlueprintResources/StandardMacros.IncrementInt` (`/Game/BASED/Player/P_Meowfficer.CanMove` Sender))
    (:`  `
      (set `/Game/BASED/Player/P_Meowfficer.CanMove` _result Sender)
      (bind _returnvalue (`GameplayStatics.GetActorOfClass` "/Game/Blueprints/Manager/BP_DialogManager.BP_DialogManager_C"))
      (bind _output_get (set `self.DialogManager` _returnvalue))
      (`/Game/Blueprints/Manager/BP_DialogManager.ShowDialog` _output_get (`self.StartRowID`) Sender))))

(event `self.SetInteractStatus`
  (params (isInteractable :type Boolean))
  (set `self.Is Interactable` isInteractable))

(event `self.UpdateHighlight`
  (params (highlightActive :type Boolean))
  ; Highlight
  (if highlightActive
    (`MeshComponent.SetOverlayMaterial` (`self.Mesh`) "/Game/GameArt/Materials/Outline/MI_InteractOutline.MI_InteractOutline")
    (else
      (`MeshComponent.SetOverlayMaterial` (`self.Mesh`) null))))

(fn `ReturnInteractStatus`
  (returns (isInteractable :type Boolean))
  (return (`self.Is Interactable`)))

(fn `ReturnSolvedStatus`
  (returns (Solved :type Boolean))
  (return (`self.Solved`)))

(fn `UserConstructionScript`)