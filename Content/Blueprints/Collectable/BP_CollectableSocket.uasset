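; Interactable puzzle socket where the P_Meowfficer player places a held collectible, or picks the placed one back up when empty-handed.
; A placed item snaps to CollectableScene; if its ID matches NeededID, the socket marks itself solved and messages ActorToReact.
; The item's OnCollected dispatcher clears the socket and reverts that state.
; Preassigned items attach on construction and BeginPlay, and an overlay material provides highlighting.
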(event `self.ReceiveBeginPlay`
  ; If Construction Script zickt rum uwu
  (bind _currentcollectible (`self.CurrentCollectible`)
    (:`then`
      (`self.K2_AttachToComponent` _currentcollectible (`self.CollectableScene`) "None" "SnapToTarget" "KeepRelative" "KeepWorld" true)
      (add `/Game/Blueprints/Collectable/BP_Collectible.OnCollectedDispatcher` (`self.CurrentCollectible`) (`|CreateDelegate` :!event `OnCurrentCollectablePickedUp`)))
    (:`else`)))

(event `/Game/BASED/Interface/BPI_Interact.SetInteractStatus`
  (params (isInteractable :type Boolean))
  ; Change Interact Status
  (set `self.isInteractable` isInteractable)
  (message `/Game/BASED/Interface/BPI_Interact.SetInteractStatus` (`self.CurrentCollectible`) isInteractable))

(event `/Game/BASED/Interface/BPI_Interact.interact`
  (params (Sender :type "/Game/BASED/Player/P_Meowfficer Object Reference"))
  ; Interact
  (`KismetSystemLibrary.IsObjectOfSoftClass` Sender "/Game/BASED/Player/P_Meowfficer.P_Meowfficer_C"
    (:`True`
      (`self.PlayerRef`
        (:`then`
          _)
        (:`else`
          (bind _asp_meowfficer (cast `/Game/BASED/Player/P_Meowfficer` Sender))
          (bind _output_get (set `self.PlayerRef` _asp_meowfficer))))
      (`self.CurrentCollectible`
        (:`then`
          ; Can Also Interact With Socket to pick item up again
          (`/Game/BASED/Player/P_Meowfficer.HeldCollectible` _output_get
            (:`then`)
            (:`else`
              (message `/Game/BASED/Interface/BPI_Interact.interact` (`self.CurrentCollectible`) (`self.PlayerRef`)))))
        (:`else`
          (bind _heldcollectible (`/Game/BASED/Player/P_Meowfficer.HeldCollectible` _output_get)
            (:`then`
              (`self.K2_AttachToComponent` _heldcollectible (`self.CollectableScene`) "None" "SnapToTarget" "KeepRelative" "KeepWorld" true)
              (`/Game/Blueprints/Collectable/BP_Collectible.PlaceColletable` _heldcollectible)
              (bind _output_get_2 (set `self.CurrentCollectible` _heldcollectible))
              (add `/Game/Blueprints/Collectable/BP_Collectible.OnCollectedDispatcher` _output_get_2 (`|CreateDelegate` :!event `OnCurrentCollectablePickedUp`))
              (set `/Game/BASED/Player/P_Meowfficer.HeldCollectible` null (`self.PlayerRef`))
              (if (`KismetStringLibrary.EqualEqual_StrStr` (`/Game/Blueprints/Collectable/BP_Collectible.ID` (`self.CurrentCollectible`)) (`self.NeededID`))
                (set `self.Solved` true)
                (message `/Game/BASED/Interface/BPI_React.React` (`self.ActorToReact`) true)))
            (:`else`)))))))

(event `OnCurrentCollectablePickedUp`
  ; Can Put on Socket again
  (bind _currentcollectible (`self.CurrentCollectible`)
    (:`then`
      (remove `/Game/Blueprints/Collectable/BP_Collectible.OnCollectedDispatcher` _currentcollectible (`|CreateDelegate` :!event `OnCurrentCollectablePickedUp`))
      (set `self.CurrentCollectible` null)
      (`self.Solved`
        (:`then`
          (set `self.Solved` false)
          (message `/Game/BASED/Interface/BPI_React.React` (`self.ActorToReact`) false))
        (:`else`)))
    (:`else`)))

(event `/Game/BASED/Interface/BPI_Interact.UpdateHighlight`
  (params (highlightActive :type Boolean))
  (bind _staticmesh (`self.StaticMesh`))
  ; Highlight
  (if highlightActive
    (`MeshComponent.SetOverlayMaterial` _staticmesh "/Game/GameArt/Materials/Outline/MI_InteractOutline.MI_InteractOutline")
    (else
      (`MeshComponent.SetOverlayMaterial` _staticmesh null))))

(fn `ReturnInteractStatus`
  (returns (isInteractable :type Boolean))
  (bind _asp_meowfficer (cast `/Game/BASED/Player/P_Meowfficer` (`GameplayStatics.GetPlayerCharacter` 0)))
  (`/Engine/EditorBlueprintResources/StandardMacros.IsValid` (`/Game/BASED/Player/P_Meowfficer.HeldCollectible` _asp_meowfficer)
    (:`Is Valid`
      (return (`self.isInteractable`)))
    (:`Is Not Valid`
      (return false))))

(fn `ReturnSolvedStatus`
  (returns (Solved :type Boolean))
  (return (`self.Solved`)))

(fn `UserConstructionScript`
  (bind _currentcollectible (`self.CurrentCollectible`)
    (:`then`
      (`self.K2_AttachToComponent` _currentcollectible (`self.CollectableScene`) "None" "SnapToTarget" "SnapToTarget" "SnapToTarget" true))
    (:`else`)))