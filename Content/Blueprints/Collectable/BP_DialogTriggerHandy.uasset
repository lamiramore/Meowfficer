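; Interactable mobile phone ("Handy") that rings and can be answered, likely as a dialog trigger.
; A phone-ringing event plays a sound, swaps to a calling material and enables interaction after a short delay.
; Interacting signals the taken call, stops the sound, disables interaction, switches the screen off and notifies ActorsToReact.
; Interaction sets Solved, while ReturnSolvedStatus reads a separate HandySolved variable.
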(event `self.ReceiveBeginPlay`
  (add `self.OnPhoneRinging` (delegate `PhoneRing`)))

(event `PhoneRing`
  (bind _returnvalue (`GameplayStatics.SpawnSoundAtLocation` (`self.HandyRinging`) (`SceneComponent.RelativeLocation` (`self.Mesh`)) (struct) 1.0 1.0 0.0 null null))
  (set `self.NewVar` _returnvalue)
  (`PrimitiveComponent.SetMaterial` (`self.Mesh`) 0 "/Game/GameArt/Assets/PCCorner/Handy/MI_HandyCalling.MI_HandyCalling")
  (`KismetSystemLibrary.Delay` 2.0)
  (`/Game/BASED/Interface/BPI_Interact.SetInteractStatus` true))

(event `/Game/BASED/Interface/BPI_Interact.UpdateHighlight`
  (params (highlightActive :type Boolean))
  (`parent.UpdateHighlight` highlightActive))

(event `/Game/BASED/Interface/BPI_Interact.interact`
  (params (Sender :type "/Game/BASED/Player/P_Meowfficer Object Reference"))
  (`parent.interact` Sender)
  (`self.SuccsessfulTakenCall`)
  (`AudioComponent.Stop` (`self.NewVar`))
  (`/Game/BASED/Interface/BPI_Interact.SetInteractStatus` false)
  (`PrimitiveComponent.SetMaterial` (`self.Mesh`) 0 "/Game/GameArt/Assets/PCCorner/Handy/MI_HandyAus.MI_HandyAus")
  (bind _output_get (set `self.Solved` true))
  (message `/Game/BASED/Interface/BPI_React.React` (`self.ActorsToReact`) _output_get))

(fn `ReturnSolvedStatus`
  (returns (Solved :type Boolean))
  (return (`self.HandySolved`)))

(fn `UserConstructionScript`
  (`parent.UserConstructionScript`))