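; BP_Collectible is an interactable item that the P_Meowfficer pawn picks up and carries, one at a time.
; Interact plays a sound, disables mesh collision, sets itself as HeldCollectible, snaps to the pawn's CollectiblePivot, turns off shadows and calls the collected dispatcher.
; PlaceColletable plays a sound and restores shadows and collision, without detaching or clearing the held reference.
; It also exposes a settable interactable flag and a read-only Solved status.
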(event `/Game/BASED/Interface/BPI_Interact.interact`
  (params (Sender :type "/Game/BASED/Player/P_Meowfficer Object Reference"))
  (bind _mesh (`self.Mesh`))
  (bind _asp_meowfficer (cast `/Game/BASED/Player/P_Meowfficer` Sender))
  (`/Game/BASED/Player/P_Meowfficer.HeldCollectible` _asp_meowfficer
    (:`then`)
    (:`else`
      (`GameplayStatics.SpawnSound2D` (`self.CollectSound`) 1.0 1.0 0.0 null)
      (`PrimitiveComponent.SetCollisionEnabled` (`self.Mesh`) "NoCollision")
      (`KismetSystemLibrary.DelayUntilNextTick`)
      (set `/Game/BASED/Player/P_Meowfficer.HeldCollectible` self _asp_meowfficer)
      (`self.K2_AttachToComponent` (`/Game/BASED/Player/P_Meowfficer.CollectiblePivot` _asp_meowfficer) "None" "SnapToTarget" "SnapToTarget" "SnapToTarget")
      (`PrimitiveComponent.SetCastShadow` _mesh false)
      (`PrimitiveComponent.SetCollisionEnabled` _mesh "NoCollision")
      (`self.OnCollectedDispatcher`))))

(event `PlaceColletable`
  (bind _mesh (`self.Mesh`))
  ; PlaceColletable
  (`GameplayStatics.SpawnSound2D` (`self.PlaceSound`) 1.0 1.0 0.0 null)
  (`PrimitiveComponent.SetCastShadow` _mesh true)
  (`PrimitiveComponent.SetCollisionEnabled` _mesh "QueryAndPhysics"))

(event `/Game/BASED/Interface/BPI_Interact.SetInteractStatus`
  (params (isInteractable :type Boolean))
  (set `self.Is Interactable` isInteractable))

(fn `ReturnInteractStatus`
  (returns (isInteractable :type Boolean))
  (return (`self.Is Interactable`)))

(fn `ReturnSolvedStatus`
  (returns (Solved :type Boolean))
  (return (`self.Solved`)))

(fn `UserConstructionScript`)